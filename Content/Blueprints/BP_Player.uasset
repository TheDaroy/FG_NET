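; Player Blueprint that shows its network role, rocket count and health on a WBP_Role widget held by the WidgetRole component.
; BeginPlay writes the local net role to the widget as text, making each instance's role visible.
; Rocket and health change events pass new values to helper functions, which cast the component's widget to WBP_Role and update it.
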(event `self.ReceiveBeginPlay`
  (bind _aswbp_role (cast `/Game/Blueprints/UI/WBP_Role` (`WidgetComponent.GetUserWidgetObject` (`self.Widget_Role`))))
  (`/Game/Blueprints/UI/WBP_Role.SetLocalText` _aswbp_role (`KismetTextLibrary.Conv_StringToText` (`|GetEnumeratorNameAsString` (`self.GetLocalRole`)))))

(event `Key|B`
  (params (Key :type "Key Structure")))

(event `self.BP_OnNumRocketsChanged`
  (params (NewNumRockets :type Integer))
  (`self.SetNumRocketsInWidget` NewNumRockets))

(event `self.BP_OnNumHealthChanged`
  (params (NewHealth :type Integer))
  (`self.SetNumHealthWidget` NewHealth))

(fn `SetNumHealthWidget`
  (params (InHealthValue :type Integer))
  (bind _aswbp_role (cast `/Game/Blueprints/UI/WBP_Role` (`WidgetComponent.GetUserWidgetObject` (`self.Widget_Role`))))
  (`/Game/Blueprints/UI/WBP_Role.SetNumHealth` _aswbp_role InHealthValue))

(fn `SetNumRocketsInWidget`
  (params (InNumRockets :type Integer))
  (bind _aswbp_role (cast `/Game/Blueprints/UI/WBP_Role` (`WidgetComponent.GetUserWidgetObject` (`self.Widget_Role`))))
  (`/Game/Blueprints/UI/WBP_Role.SetNumRockets` _aswbp_role InNumRockets))

(fn `UserConstructionScript`)